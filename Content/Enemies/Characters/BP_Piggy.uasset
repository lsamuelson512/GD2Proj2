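; BP_Piggy is a piggy enemy that registers itself with the first-person player character.
; Shortly after BeginPlay it casts and caches the player, then increments the player's EnemyCount.
; It binds to its own OnDestroyed event, which calls EnemiesSlained on the player to report the kill.
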(event Custom|EnemyKilled
  (params (DestroyedActor :type Actor%20Object%20Reference))
  (Default|EnemiesSlained (Variables|Default|GetPlayerRef) (Variables|Default|GetAdditional)))

(event EventBeginPlay
  (Utilities|FlowControl|Delay 0.2)
  (bind _asbp_first_person_character (Utilities|Casting|CastToBP_FirstPersonCharacter (Game|GetPlayerCharacter 0)))
  (bind _output_get (Variables|Default|SetPlayerRef _asbp_first_person_character))
  (Math|Integer|IncrementInt (Variables|/Game/FirstPerson/Blueprints/BP_FirstPersonCharacter.BP_FirstPersonCharacter_C|GetEnemyCount _output_get)
    (:%20%20
      (Game|BindEventtoOnDestroyed (delegate Custom|EnemyKilled)))))

(fn ConstructionScript)