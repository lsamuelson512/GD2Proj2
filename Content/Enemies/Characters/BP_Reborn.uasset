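; BP_Reborn is an enemy character that throws a lobbed projectile at the player.
; ThrowLob spawns BP_LobProjectile at the mesh's Projectile socket, enables collision, then after a zero-length delay launches it with a velocity-change impulse.
; FindVelocity derives flight time from horizontal distance and computes a gravity-based arc toward player 0, ignoring height difference and adding a gravity term to horizontal speed.
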(event Custom|ThrowLob
  (bind _returnvalue (Game|SpawnActorfromClass "/Game/Enemies/Projectiles/BP_LobProjectile.BP_LobProjectile_C" (Transformation|GetSocketTransform (Variables|Character|GetMesh) "Projectile" "RTS_World") "AlwaysSpawn" "MultiplyWithRoot" 0 0))
  (bind _output_get (Variables|Default|SetProjectileRef _returnvalue))
  (Collision|SetCollisionEnabled (Variables|/Game/Enemies/Projectiles/BP_LobProjectile.BP_LobProjectile_C|GetCollision _output_get) "QueryAndPhysics")
  (Collision|SetCollisionEnabled (Variables|/Game/Enemies/Projectiles/BP_LobProjectile.BP_LobProjectile_C|GetProjectile _output_get) "QueryAndPhysics")
  (Utilities|FlowControl|Delay 0.0)
  (Physics|AddImpulse (Variables|/Game/Enemies/Projectiles/BP_LobProjectile.BP_LobProjectile_C|GetProjectile _output_get) (CallFunction|FindVelocity _output_get) "None" true))

(fn ConstructionScript)

(fn FindVelocity
  (params (Projectile :type BP%20Lob%20Projectile%20Object%20Reference))
  (bind _returnvalue (Game|GetPlayerCharacter 0))
  (bind _returnvalue_2 (Transformation|GetActorLocation Projectile))
  (bind _returnvalue_3 (Transformation|GetActorLocation _returnvalue))
  (bind _returnvalue_4 (Math|Vector|GetUnitDirection(Vector) _returnvalue_2 _returnvalue_3))
  (bind _returnvalue_5 (- _returnvalue_2 _returnvalue_3))
  (bind _returnvalue_6 (Math|Vector|VectorLength (Math|Vector|MakeVector (.x _returnvalue_5) (.y _returnvalue_5) 0.0)))
  (bind _returnvalue_7 (/ _returnvalue_6 1e+03))
  (bind _returnvalue_8 (Math|Float|Square _returnvalue_7))
  (bind _returnvalue_9 (* 0.5 -9.8e+02 _returnvalue_8))
  (bind _returnvalue_10 (- _returnvalue_6 _returnvalue_9))
  (bind _returnvalue_11 (/ _returnvalue_10 _returnvalue_7))
  (bind _returnvalue_12 (* _returnvalue_11 (Math|Vector|MakeVector (.x _returnvalue_4) (.y _returnvalue_4) 0.0)))
  (return (Math|Vector|MakeVector (.x _returnvalue_12) (.y _returnvalue_12) (* _returnvalue_7 -1.0 -9.8e+02 0.5))))