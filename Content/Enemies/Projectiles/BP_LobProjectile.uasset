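; BP_LobProjectile is an enemy projectile that damages the player through a direct hit or an area of effect.
; A collision hit on BP_FirstPersonCharacter deals full damage via its damageable component and destroys the projectile immediately.
; Any other hit deals half damage to a player overlapping the AOE, gated by DoOnce, then destroys the projectile after a short delay.
; The construction script enables query and physics collision.
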(event OnComponentHit(Collision)
  (params (HitComponent :type Primitive%20Component%20Object%20Reference) (OtherActor :type Actor%20Object%20Reference) (OtherComp :type Primitive%20Component%20Object%20Reference) (NormalImpulse :type Vector :default "0, 0, 0") (Hit :type Hit%20Result%20Structure%20%28by%20ref%29))
  (bind _asbp_first_person_character (Utilities|Casting|CastToBP_FirstPersonCharacter OtherActor)
    (:then
      (Default|Damaged (Variables|/Game/FirstPerson/Blueprints/BP_FirstPersonCharacter.BP_FirstPersonCharacter_C|GetBP_Damagable _asbp_first_person_character) (Variables|Default|GetDamage%20Amount))
      (Actor|DestroyActor))
    (:CastFailed
      (for _array_element (Collision|GetOverlappingActors (Variables|Default|GetAOE) "/Game/FirstPerson/Blueprints/BP_FirstPersonCharacter.BP_FirstPersonCharacter_C" :!class /Script/Engine.PrimitiveComponent)
        (Utilities|FlowControl|DoOnce false
          (:Completed
            (Default|Damaged (Actor|GetComponentbyClass _array_element "/Game/FirstPerson/Blueprints/DamageSystem/BP_Damagable.BP_Damagable_C") (/ (Variables|Default|GetDamage%20Amount) 2.0)))))
      (Utilities|FlowControl|Delay 0.2)
      (Actor|DestroyActor))))

(fn ConstructionScript
  (Collision|SetCollisionEnabled (Variables|Default|GetCollision) "QueryAndPhysics"))